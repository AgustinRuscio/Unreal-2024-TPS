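; BP_Enemy is an enemy Blueprint whose construction script equips it with a pistol, rifle or shotgun.
; EnemyWeaponType is passed to ShootComponent and selects a setter that assigns the matching skeletal mesh to WeaponMesh and the weapon's fire animation to GunShootAnim.
; The script then hands the mesh component and animation to ShootComponent, so the loadout is resolved at construction.
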(fn `Set Pistol`
  (`SkeletalMeshComponent.SetSkeletalMeshAsset` (`self.WeaponMesh`) "/Game/MilitaryWeapSilver/Weapons/Pistols_A.Pistols_A")
  (set `self.GunShootAnim` "/Game/MilitaryWeapSilver/Weapons/Animations/Fire_Pistol_W.Fire_Pistol_W"))

(fn `Set Rifle`
  (`SkeletalMeshComponent.SetSkeletalMeshAsset` (`self.WeaponMesh`) "/Game/MilitaryWeapSilver/Weapons/Assault_Rifle_A.Assault_Rifle_A")
  (set `self.GunShootAnim` "/Game/MilitaryWeapSilver/Weapons/Animations/Fire_Rifle_W.Fire_Rifle_W"))

(fn `Set Shotgun`
  (`SkeletalMeshComponent.SetSkeletalMeshAsset` (`self.WeaponMesh`) "/Game/MilitaryWeapSilver/Weapons/Shotgun_A.Shotgun_A")
  (set `self.GunShootAnim` "/Game/MilitaryWeapSilver/Weapons/Animations/Fire_Shotgun_W.Fire_Shotgun_W"))

(fn `UserConstructionScript`
  (bind _enemyweapontype (`self.EnemyWeaponType`))
  (`ShootComponent.SetCurrentWeaponType` (`self.ShootComponent`) _enemyweapontype)
  (switch `EWeaponType` _enemyweapontype
    (:`Pistol`
      (`self.Set Pistol`))
    (:`Rifle`
      (`self.Set Rifle`))
    (:`Shotgun`
      (`self.Set Shotgun`)))
  (`ShootComponent.SetWeaponSkeleton` (`self.ShootComponent`) (`self.WeaponMesh`) (`self.GunShootAnim`)))